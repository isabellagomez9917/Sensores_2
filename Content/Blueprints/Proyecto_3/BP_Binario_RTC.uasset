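; BP_Binario_RTC is a light actor whose brightness follows a seconds value received over UDP, apparently from a real-time clock.
; It enables player input on BeginPlay, and the G key toggles a receive socket on a hardcoded IP and port.
; The first byte of each packet becomes Seconds, which RTCcustom maps with a clamped range onto the PointLight's intensity.
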(event OnReceivedBytes(UDP)
  (params (Bytes :type Array%20of%20Bytes) (IPAddress :type String))
  (Variables|Default|Setseconds (Math|Conversions|ToFloat(Byte) (Utilities|Array|Get(acopy) Bytes)))
  (CallFunction|RTCcustom))

(event Custom|RTCcustom
  ;[1 1 1] RTC funcionality
  (Rendering|Components|Light|SetIntensity (Variables|Default|GetPointLight) (Math|Float|MapRangeClamped (Variables|Default|Getseconds) 0.0 59.0 0.0 1e+03)))

(event EventBeginPlay
  (Input|EnableInput (Game|GetPlayerController 0)))

(event Input|KeyboardEvents|G
  (params (Key :type Key%20Structure :default "None"))
  (bind _udp (Variables|Default|GetUDP))
  (:Pressed
    (Utilities|FlowControl|FlipFlop
      (:A
        (Class|UDPComponent|OpenReceiveSocket _udp "192.168.1.103" 30)
        (Development|PrintString "Socket 2: opened"))
      (:B
        (Class|UDPComponent|CloseReceiveSocket _udp)
        (Development|PrintString "Socket 2: closed")))))

(fn ConstructionScript)