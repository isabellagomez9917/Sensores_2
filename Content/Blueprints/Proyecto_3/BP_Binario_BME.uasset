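; Test Blueprint that receives binary UDP data and prints it as a float on screen.
; The G key alternates between opening a receive socket on a hardcoded IP and port and closing it, with input enabled for player 0 on BeginPlay.
; Each received packet is converted with BytesToFloat and printed with the sender's IP.
; An empty custom event and a disconnected first-byte print are left unused.
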(event OnReceivedBytes(UDP)
  (params (Bytes :type Array%20of%20Bytes) (IPAddress :type String))
  (Development|PrintString (Utilities|String|Append (Utilities|String|ToString(Float) (Class|Serial|BytestoFloat Bytes)) " from IP: " IPAddress)))

(event Custom|CustomEvent
  (params (Bytes :type Array%20of%20Bytes) (IPAddress :type String)))

(event EventBeginPlay
  (Input|EnableInput (Game|GetPlayerController 0)))

(event Input|KeyboardEvents|G
  (params (Key :type Key%20Structure :default "None"))
  (bind _udp (Variables|Default|GetUDP))
  (:Pressed
    (Utilities|FlowControl|FlipFlop
      (:A
        (bind _returnvalue (Class|UDPComponent|OpenReceiveSocket _udp "192.168.1.103" 30))
        (Development|PrintString (Utilities|String|ToString(Boolean) _returnvalue)))
      (:B
        (Class|UDPComponent|CloseReceiveSocket _udp)
        (Development|PrintString "Socket closed")))))

(fn ConstructionScript)