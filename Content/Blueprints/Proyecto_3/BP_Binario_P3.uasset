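; Actor that polls an ESP32 over a serial COM port and drives scene lighting and chair materials from its clock and BME280 readings.
; BeginPlay adds the port widget and creates dynamic chair materials; events open and close the port.
; Tick, after a delay, writes a request byte and parses seven bytes into seconds, minutes and a float.
; The float tints PointLight2 between red and blue, while seconds and minutes set each chair's emissive parameter.
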(event Custom|Open%20Port%20Binario
  ;[0.2619 0.2638 0.3229] Open/Close ports ESP32
  (bind (_bopened _returnvalue) (Class|Serial|OpenComPort (Variables|Default|GetPortBinario) (Variables|Default|GetBaudBinario)))
  (if _bopened
    (bind _output_get (Variables|Default|SetESP32 _returnvalue))
    (Development|PrintString "Puerto abierto" true true "(R=0.000000,G=0.660000,B=1.000000,A=1.000000)" 5.0)
    (Class|Serial|Flush _output_get)))

(event Custom|Close%20Port%20Binario
  (bind _esp32 (Variables|Default|GetESP32))
  ;[0.2619 0.2638 0.3229] Open/Close ports ESP32
  (Utilities|IsValid _esp32
    (:Is%20Valid
      (Class|Serial|Close _esp32)
      (Development|PrintString "Puerto Cerrado"))))

(event Custom|BME
  ;[1 1 1] BME funcionality
  (Rendering|Components|Light|SetLightColor (Variables|Default|GetPointLight2) (Math|Color|Lerp(LinearColor) "(R=1.000000,G=0.000000,B=0.018653,A=1.000000)" "(R=0.000000,G=0.079093,B=1.000000,A=1.000000)" (Math|Float|MapRangeClamped (Variables|Default|GetBME280) 4e+01 6e+01 0.0 1.0)) true))

(event Custom|RTC
  ;[1 1 1] RTC funcionality
  (Rendering|Material|SetScalarParameterValue (Variables|Default|GetMaterialSillaS) "Emmisive Color" (Math|Float|MapRangeClamped (Variables|Default|Getseconds) 0.0 59.0 0.0 0.1) :!class /Script/Engine.MaterialInstanceDynamic)
  (Rendering|Material|SetScalarParameterValue (Variables|Default|GetMaterialSillaM) "Emmisive Color" (Math|Float|MapRangeClamped (Variables|Default|Getminutes) 0.0 59.0 0.0 0.1) :!class /Script/Engine.MaterialInstanceDynamic))

(event EventBeginPlay
  ;[0.2619 0.2638 0.3229] Open/Close ports ESP32
  (bind _returnvalue (UserInterface|CreateWidget "/Game/Blueprints/Proyecto_2/BPW_PortBinario_P2.BPW_PortBinario_P2_C"))
  (UserInterface|Viewport|AddtoViewport _returnvalue 0)
  (Variables|/Script/Engine.PlayerController|SetbShowMouseCursor (Game|GetPlayerController 0) true)
  (bind _returnvalue_2 (Rendering|Material|CreateDynamicMaterialInstance "/Game/StarterContent/Props/Materials/M_Chair.M_Chair" "None" :!class /Script/Engine.KismetMaterialLibrary))
  (Variables|Default|SetMaterialSillaS _returnvalue_2)
  (Rendering|Material|SetMaterial (Variables|Default|GetChair) 0 (Variables|Default|GetMaterialSillaS))
  (bind _returnvalue_3 (Rendering|Material|CreateDynamicMaterialInstance "/Game/StarterContent/Props/Materials/M_Chair.M_Chair" "None" :!class /Script/Engine.KismetMaterialLibrary))
  (Variables|Default|SetMaterialSillaM _returnvalue_3)
  (Rendering|Material|SetMaterial (Variables|Default|GetChair2) 0 (Variables|Default|GetMaterialSillaM)))

(event EventEndPlay
  (params (EndPlayReason :type EEndPlayReason%20Enum :default "Destroyed"))
  (bind _esp32 (Variables|Default|GetESP32))
  ;[0.2619 0.2638 0.3229] Open/Close ports ESP32
  (Utilities|IsValid _esp32
    (:Is%20Valid
      (Class|Serial|Close _esp32)
      (Development|PrintString "Puerto NO abierto"))))

(event EventTick
  (params (DeltaSeconds :type Float%20%28single-precision%29))
  (bind _esp32 (Variables|Default|GetESP32))
  (Utilities|IsValid _esp32
    (:Is%20Valid
      (Utilities|FlowControl|Delay 0.2)
      (bind _returnvalue (Class|Serial|WriteByte _esp32))
      ;[0.2619 0.2638 0.3229] Slider connected to DigitalDataRead_SlideSwitch_Binario.ino
      (if _returnvalue
        (bind _returnvalue_2 (Class|Serial|ReadBytes _esp32 7))
        (if (== (Utilities|Array|Length _returnvalue_2) 7)
          (for (_array_element _array_index) _returnvalue_2
            (if (< _array_index 3)
              (Variables|Default|SetBytesNumber (Utilities|String|Append (Variables|Default|GetBytesNumber) "," (Utilities|String|ToString(Byte) _array_element)))))
          (Variables|Default|SetBytesNumber (Utilities|String|Append (Variables|Default|GetBytesNumber) "---" (Utilities|String|ToString(Float) (Class|Serial|BytestoFloat (Utilities|Array|MakeArray (Utilities|Array|Get(acopy) _returnvalue_2 3) (Utilities|Array|Get(acopy) _returnvalue_2 4) (Utilities|Array|Get(acopy) _returnvalue_2 5) (Utilities|Array|Get(acopy) _returnvalue_2 6))))))
          (Variables|Default|Setseconds (Math|Conversions|ToFloat(Byte) (Utilities|Array|Get(acopy) _returnvalue_2)))
          (Variables|Default|Setminutes (Math|Conversions|ToFloat(Byte) (Utilities|Array|Get(acopy) _returnvalue_2 1)))
          (Variables|Default|SetBME280 (Class|Serial|BytestoFloat (Utilities|Array|MakeArray (Utilities|Array|Get(acopy) _returnvalue_2 3) (Utilities|Array|Get(acopy) _returnvalue_2 4) (Utilities|Array|Get(acopy) _returnvalue_2 5) (Utilities|Array|Get(acopy) _returnvalue_2 6))))
          (Development|PrintString (Variables|Default|GetBytesNumber))
          (CallFunction|BME)
          (CallFunction|RTC))
        (Variables|Default|SetBytesNumber "")))))

(fn ConstructionScript)