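; BP_ASCII is an actor that drives a point light's intensity from a potentiometer on an Arduino/ESP32 over a serial port.
; On BeginPlay it shows the BPW_PortASCII widget and mouse cursor, with custom events to open and close the COM port.
; Each Tick it reads an ASCII string from the port, converts it to float and smoothly interpolates the light intensity toward it.
; EndPlay closes any open port.
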(event Custom|Open%20Port%20ASCII
  ;[0.2619 0.2638 0.3229] Open/Close ports with Arduino and ESP32
  (bind (_bopened _returnvalue) (Class|Serial|OpenComPort (Variables|Default|GetPortASCII) (Variables|Default|GetBaudASCII)))
  (if _bopened
    (bind _output_get (Variables|Default|SetESP32 _returnvalue))
    (Development|PrintString "Puerto abierto" true true "(R=0.000000,G=0.660000,B=1.000000,A=1.000000)" 5.0)
    (Class|Serial|Flush _output_get)))

(event Custom|Close%20Port%20ASCII
  (bind _esp32 (Variables|Default|GetESP32))
  ;[0.2619 0.2638 0.3229] Open/Close ports with Arduino and ESP32
  (Utilities|IsValid _esp32
    (:Is%20Valid
      (Class|Serial|Close _esp32)
      (Development|PrintString "Puerto Cerrado"))))

(event EventEndPlay
  (params (EndPlayReason :type EEndPlayReason%20Enum :default "Destroyed"))
  (bind _esp32 (Variables|Default|GetESP32))
  ;[0.2619 0.2638 0.3229] Open/Close ports with Arduino and ESP32
  (Utilities|IsValid _esp32
    (:Is%20Valid
      (Class|Serial|Close _esp32)
      (Development|PrintString "Puerto NO abierto"))))

(event EventBeginPlay
  ;[0.2619 0.2638 0.3229] Open/Close ports with Arduino and ESP32
  (bind _returnvalue (UserInterface|CreateWidget "/Game/Blueprints/Proyecto_1/BPW_PortASCII.BPW_PortASCII_C"))
  (UserInterface|Viewport|AddtoViewport _returnvalue 0)
  (Variables|/Script/Engine.PlayerController|SetbShowMouseCursor (Game|GetPlayerController 0) true))

(event EventTick
  (params (DeltaSeconds :type Float%20%28single-precision%29))
  (bind _esp32 (Variables|Default|GetESP32))
  (bind _pointlight (Variables|Default|GetPointLight))
  ;[0.2619 0.2638 0.3229] Potenciometer connected to AnaloglRead.ino No keyboard needed
  (Utilities|IsValid _esp32
    (:Is%20Valid
      (bind _returnvalue (Class|Serial|ReadString _esp32))
      (Rendering|Components|Light|SetIntensity _pointlight (Math|Interpolation|FInterpTo (Variables|/Script/Engine.LightComponentBase|GetIntensity _pointlight) (Math|Conversions|ToFloat(Integer) _returnvalue) DeltaSeconds 2.0)))))

(fn ConstructionScript)