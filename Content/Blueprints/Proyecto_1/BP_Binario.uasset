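; BP_Binario is an Arduino/ESP32 serial test actor that switches a point light from a hardware slide switch.
; On BeginPlay it shows a port widget and mouse cursor, with events to open and close the COM port.
; Tick reads one byte from the open port, lighting PointLight2 when it matches ASCII '1' and turning it off for any other byte.
; EndPlay closes the port.
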(event Custom|Open%20Port%20Binario
  ;[0.2619 0.2638 0.3229] Open/Close ports with Arduino and ESP32
  (bind (_bopened _returnvalue) (Class|Serial|OpenComPort (Variables|Default|GetPortBinario) 9600))
  (if _bopened
    (bind _output_get (Variables|Default|SetArduino _returnvalue))
    (Development|PrintString "Puerto abierto" true true "(R=0.000000,G=0.660000,B=1.000000,A=1.000000)" 5.0)
    (Class|Serial|Flush _output_get)))

(event Custom|Close%20Port%20Binario
  (bind _arduino (Variables|Default|GetArduino))
  ;[0.2619 0.2638 0.3229] Open/Close ports with Arduino and ESP32
  (Utilities|IsValid _arduino
    (:Is%20Valid
      (Class|Serial|Close _arduino)
      (Development|PrintString "Puerto Cerrado"))))

(event EventBeginPlay
  ;[0.2619 0.2638 0.3229] Open/Close ports with Arduino and ESP32
  (bind _returnvalue (UserInterface|CreateWidget "/Game/Blueprints/Proyecto_1/BPW_PortBinario.BPW_PortBinario_C"))
  (UserInterface|Viewport|AddtoViewport _returnvalue 0)
  (Variables|/Script/Engine.PlayerController|SetbShowMouseCursor (Game|GetPlayerController 0) true))

(event EventEndPlay
  (params (EndPlayReason :type EEndPlayReason%20Enum :default "Destroyed"))
  (bind _arduino (Variables|Default|GetArduino))
  ;[0.2619 0.2638 0.3229] Open/Close ports with Arduino and ESP32
  (Utilities|IsValid _arduino
    (:Is%20Valid
      (Class|Serial|Close _arduino)
      (Development|PrintString "Puerto NO abierto"))))

(event EventTick
  (params (DeltaSeconds :type Float%20%28single-precision%29))
  (bind _arduino (Variables|Default|GetArduino))
  ;[0.2619 0.2638 0.3229] Slider connected to DigitalDataRead_SlideSwitch_Binario.ino
  (Utilities|IsValid _arduino
    (:Is%20Valid
      (bind (_bsuccess _returnvalue) (Class|Serial|ReadByte _arduino)) ; Lee 1 byte
      (if _bsuccess
        (Development|PrintString (Utilities|String|ToString(Byte) _returnvalue))
        (if (Utilities|Enum|Equal(Enum) (Utilities|String|ToString(Byte) _returnvalue) "49")
          (Rendering|Components|Light|SetIntensity (Variables|Default|GetPointLight2) 2.5e+03)
          (else
            (Rendering|Components|Light|SetIntensity (Variables|Default|GetPointLight2) 0.0)))))))

(fn ConstructionScript)